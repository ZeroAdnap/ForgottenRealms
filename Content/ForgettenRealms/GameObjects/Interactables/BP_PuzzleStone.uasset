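; Pushable puzzle stone that slides along the X or Y axis when interacted with, unless already moving or locked on a pressure plate.
; Four side overlap boxes set the push direction, and a box trace picks the destination: trace end, or hit point followed by a slight back-off.
; MoveComponentTo animates the slide, which StopMovement can halt.
; Two trigger volumes reveal the interact icon, then its hotkey and text.
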(event OnComponentBeginOverlap(PushBoxYPositive)
  (params (OverlappedComponent :type Primitive%20Component%20Object%20Reference) (OtherActor :type Actor%20Object%20Reference) (OtherComp :type Primitive%20Component%20Object%20Reference) (OtherBodyIndex :type Integer) (bFromSweep :type Boolean) (SweepResult :type Hit%20Result%20Structure%20%28by%20ref%29))
  ;[1 1 1] Y Axis Collision (Positive)
  (Variables|Default|SetDirection%20to%20Push "0.000000,250.000000,0.000000"))

(event OnComponentBeginOverlap(PushBoxXPositive)
  (params (OverlappedComponent :type Primitive%20Component%20Object%20Reference) (OtherActor :type Actor%20Object%20Reference) (OtherComp :type Primitive%20Component%20Object%20Reference) (OtherBodyIndex :type Integer) (bFromSweep :type Boolean) (SweepResult :type Hit%20Result%20Structure%20%28by%20ref%29))
  ;[1 1 1] X Axis Collision (Positive)
  (Variables|Default|SetDirection%20to%20Push "250.000000,0.000000,0.000000"))

(event OnComponentEndOverlap(InteractPrompt)
  (params (OverlappedComponent :type Primitive%20Component%20Object%20Reference) (OtherActor :type Actor%20Object%20Reference) (OtherComp :type Primitive%20Component%20Object%20Reference) (OtherBodyIndex :type Integer))
  (bind _aswb_interact_icon (Utilities|Casting|CastToWB_InteractIcon (UserInterface|GetWidget (Variables|Default|GetWidget))))
  (Widget|SetVisibility (Variables|/Game/ForgettenRealms/HUD/WB_InteractIcon.WB_InteractIcon_C|GetHotkey _aswb_interact_icon) "Hidden"))

(event OnComponentBeginOverlap(PushBoxXNegative)
  (params (OverlappedComponent :type Primitive%20Component%20Object%20Reference) (OtherActor :type Actor%20Object%20Reference) (OtherComp :type Primitive%20Component%20Object%20Reference) (OtherBodyIndex :type Integer) (bFromSweep :type Boolean) (SweepResult :type Hit%20Result%20Structure%20%28by%20ref%29))
  ;[1 1 1] X Axis Collision (Negative)
  (Variables|Default|SetDirection%20to%20Push "-250.000000,0.000000,0.000000"))

(event OnComponentBeginOverlap(PushBoxYNegative)
  (params (OverlappedComponent :type Primitive%20Component%20Object%20Reference) (OtherActor :type Actor%20Object%20Reference) (OtherComp :type Primitive%20Component%20Object%20Reference) (OtherBodyIndex :type Integer) (bFromSweep :type Boolean) (SweepResult :type Hit%20Result%20Structure%20%28by%20ref%29))
  ;[1 1 1] Y Axis Collision (Positive)
  (Variables|Default|SetDirection%20to%20Push "0.000000,-250.000000,0.000000"))

(event OnComponentBeginOverlap(VisiblePrompt)
  (params (OverlappedComponent :type Primitive%20Component%20Object%20Reference) (OtherActor :type Actor%20Object%20Reference) (OtherComp :type Primitive%20Component%20Object%20Reference) (OtherBodyIndex :type Integer) (bFromSweep :type Boolean) (SweepResult :type Hit%20Result%20Structure%20%28by%20ref%29))
  (bind _widget (Variables|Default|GetWidget))
  (Utilities|IsValid (Variables|Default|GetWidget)
    (:Is%20Valid
      (if (== (Utilities|GetClass OtherActor) "/Game/ForgettenRealms/Player/BP_WukongPlayer.BP_WukongPlayer_C")
        (Rendering|SetVisibility _widget true false)
        (Class|WidgetComponent|SetTickMode _widget "Enabled")))))

(event OnComponentEndOverlap(VisiblePrompt)
  (params (OverlappedComponent :type Primitive%20Component%20Object%20Reference) (OtherActor :type Actor%20Object%20Reference) (OtherComp :type Primitive%20Component%20Object%20Reference) (OtherBodyIndex :type Integer))
  (bind _widget (Variables|Default|GetWidget))
  (Utilities|IsValid (Variables|Default|GetWidget)
    (:Is%20Valid
      (Rendering|SetVisibility _widget false false)
      (Class|WidgetComponent|SetTickMode _widget "Automatic"))))

(event OnComponentBeginOverlap(InteractPrompt)
  (params (OverlappedComponent :type Primitive%20Component%20Object%20Reference) (OtherActor :type Actor%20Object%20Reference) (OtherComp :type Primitive%20Component%20Object%20Reference) (OtherBodyIndex :type Integer) (bFromSweep :type Boolean) (SweepResult :type Hit%20Result%20Structure%20%28by%20ref%29))
  (bind _aswb_interact_icon (Utilities|Casting|CastToWB_InteractIcon (UserInterface|GetWidget (Variables|Default|GetWidget))))
  (Widget|SetVisibility (Variables|/Game/ForgettenRealms/HUD/WB_InteractIcon.WB_InteractIcon_C|GetHotkey _aswb_interact_icon) "Visible"))

(event Custom|StopMovement
  (bind _returnvalue (Transformation|GetActorLocation))
  (bind _direction_to_push (Variables|Default|GetDirection%20to%20Push))
  (bind _returnvalue_2 (/ _direction_to_push 35.0))
  (bind _returnvalue_3 (- _returnvalue _returnvalue_2))
  ;[1 1 1] Stop movement immediately
  (Utilities|FlowControl|Sequence
    (:then_0
      ;[1 1 1] Object in the way, move to hit location
      (Components|MoveComponentTo (Variables|Transformation|GetRootComponent) (Utilities|MakeHitVector (.x (.Location (Collision|BreakHitResult (stale EventInteract _outhit)))) (.y (.Location (Collision|BreakHitResult (stale EventInteract _outhit))))) "0, 0, 0" false false 1.5 false) ; enters at Stop
    )
    (:then_1
      ;[1 1 1] No object in the way, move to line trace location
      (Components|MoveComponentTo (Variables|Transformation|GetRootComponent) (Utilities|MakeHitVector (.x (.TraceEnd (Collision|BreakHitResult (stale EventInteract _outhit)))) (.y (.TraceEnd (Collision|BreakHitResult (stale EventInteract _outhit))))) "0, 0, 0" false false 1.5 false) ; enters at Stop
    )))

(event EventInteract
  (bind _returnvalue (Transformation|GetActorLocation))
  (bind _returnvalue_2 (Transformation|GetActorLocation))
  (bind _direction_to_push (Variables|Default|GetDirection%20to%20Push))
  (bind _returnvalue_3 (/ _direction_to_push 35.0))
  (bind _returnvalue_4 (- _returnvalue_2 _returnvalue_3))
  ;[1 1 1] On pressure plate?
  (if (not (Variables|Default|GetLockedOnPlate))
    ;[1 1 1] Already moving?
    (if (not (Variables|Default|GetMoving?))
      ;[1 1 1] Set as moving
      (Variables|Default|SetMoving? true)
      ;[1 1 1] Trace for objects in the path
      (bind (_outhit _returnvalue_5) (Collision|BoxTraceByChannel (Math|Vector|MakeVector (.x _returnvalue) (.y _returnvalue) (+ (.z _returnvalue) (.z (Utilities|ObjectExtent)) 5.0)) (Utilities|MakeDirectionYVector) (* (Utilities|ObjectExtent) 0.75) "0, 0, 0" "TraceTypeQuery1" false 0 "None"))
      ;[1 1 1] Play stone drag sound
      (Audio|PlaySoundatLocation "/Game/ForgettenRealms/FX/SoundFX/StonePush.StonePush" (Transformation|GetActorLocation) "0, 0, 0" 1.0 1.0 0.4 0 0 0 0)
      (if _returnvalue_5
        (Variables|Default|SetHit%20Location (Utilities|MakeHitVector (.x (.Location (Collision|BreakHitResult _outhit))) (.y (.Location (Collision|BreakHitResult _outhit)))))
        ;[1 1 1] Object in the way, move to hit location
        (Components|MoveComponentTo (Variables|Transformation|GetRootComponent) (Utilities|MakeHitVector (.x (.Location (Collision|BreakHitResult _outhit))) (.y (.Location (Collision|BreakHitResult _outhit)))) "0, 0, 0" false false 1.5 false)
        (Components|MoveComponentTo (Variables|Transformation|GetRootComponent) (Math|Vector|MakeVector (.x _returnvalue_4) (.y _returnvalue_4) (.z (Transformation|GetActorLocation))) "0, 0, 0" false false 0.2 false)
        (else
          ;[1 1 1] No object in the way, move to line trace location
          (Components|MoveComponentTo (Variables|Transformation|GetRootComponent) (Utilities|MakeHitVector (.x (.TraceEnd (Collision|BreakHitResult _outhit))) (.y (.TraceEnd (Collision|BreakHitResult _outhit)))) "0, 0, 0" false false 1.5 false)))
      ;[1 1 1] Reset moving variable
      (Variables|Default|SetMoving? false))))

(event EventBeginPlay
  (bind _widget (Variables|Default|GetWidget))
  (Utilities|IsValid (Variables|Default|GetWidget)
    (:Is%20Valid
      (Rendering|SetVisibility _widget false false)
      (Class|WidgetComponent|SetTickMode _widget "Automatic")
      (bind _aswb_interact_icon (Utilities|Casting|CastToWB_InteractIcon (UserInterface|GetWidget (Variables|Default|GetWidget))))
      (Variables|/Game/ForgettenRealms/HUD/WB_InteractIcon.WB_InteractIcon_C|SetInteractText _aswb_interact_icon (Variables|Default|GetInteractText)))))

(fn ConstructionScript)