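; BP_RunePuzzle is a runestone combination puzzle that completes a quest when solved.
; SetPasswordInteger stores each changed stone's interaction count, minus one, at that stone's index in PasswordEntered.
; Tick polls PasswordsEqual and, once true, lights a target rune and completes the quest on the Wukong player, guarded by DoOnce.
; PasswordsEqual contains a three-slot comparison against PasswordAnswer, but those nodes appear unconnected.
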(event Custom|SetPasswordInteger
  (params (RunestoneChanged :type BP%20Child%20Runestone%20Object%20Reference) (TimesInteracted :type Integer))
  (Utilities|Array|SetArrayElem (Variables|Default|GetPasswordEntered) (Utilities|Array|FindItem (Variables|Default|GetRunestones) RunestoneChanged) (- TimesInteracted 1)))

(event EventTick
  (params (DeltaSeconds :type Float%20%28single-precision%29))
  (if (Utilities|PasswordsEqual?)
    (Utilities|FlowControl|DoOnce false
      (:Completed
        (Default|LightRune (Variables|Default|GetRunestoneToLight))
        (bind _asbp_wukong_player (Utilities|Casting|CastToBP_WukongPlayer (Game|Player|GetPlayerPawn 0)))
        (Default|CompleteQuest (Variables|/Game/ForgettenRealms/Player/BP_WukongPlayer.BP_WukongPlayer_C|GetSYS_Quests _asbp_wukong_player) (Variables|Default|GetQuestToComplete))))))

(fn ConstructionScript)