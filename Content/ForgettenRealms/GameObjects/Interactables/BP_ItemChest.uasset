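; One-time interactable item chest that grants the Wukong player either a bomb or a random item.
; Overlap volumes reveal the interact widget and its hotkey prompt, which is destroyed on use.
; Interacting runs a timeline that slides and turns the player to the chest, then disables input and hides the staff during the opening montage, sound and chest animation.
; When the montage ends, control returns and an item widget displays the reward.
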(event OnComponentBeginOverlap(VisiblePrompt)
  (params (OverlappedComponent :type Primitive%20Component%20Object%20Reference) (OtherActor :type Actor%20Object%20Reference) (OtherComp :type Primitive%20Component%20Object%20Reference) (OtherBodyIndex :type Integer) (bFromSweep :type Boolean) (SweepResult :type Hit%20Result%20Structure%20%28by%20ref%29))
  (bind _widget (Variables|Default|GetWidget))
  (Utilities|IsValid (Variables|Default|GetWidget)
    (:Is%20Valid
      (if (== (Utilities|GetClass OtherActor) "/Game/ForgettenRealms/Player/BP_WukongPlayer.BP_WukongPlayer_C")
        (Rendering|SetVisibility _widget true false)
        (Class|WidgetComponent|SetTickMode _widget "Enabled")))))

(event OnComponentEndOverlap(VisiblePrompt)
  (params (OverlappedComponent :type Primitive%20Component%20Object%20Reference) (OtherActor :type Actor%20Object%20Reference) (OtherComp :type Primitive%20Component%20Object%20Reference) (OtherBodyIndex :type Integer))
  (bind _widget (Variables|Default|GetWidget))
  (Utilities|IsValid (Variables|Default|GetWidget)
    (:Is%20Valid
      (Rendering|SetVisibility _widget false false)
      (Class|WidgetComponent|SetTickMode _widget "Automatic"))))

(event OnComponentBeginOverlap(InteractPrompt)
  (params (OverlappedComponent :type Primitive%20Component%20Object%20Reference) (OtherActor :type Actor%20Object%20Reference) (OtherComp :type Primitive%20Component%20Object%20Reference) (OtherBodyIndex :type Integer) (bFromSweep :type Boolean) (SweepResult :type Hit%20Result%20Structure%20%28by%20ref%29))
  (Utilities|IsValid (Variables|Default|GetWidget)
    (:Is%20Valid
      (bind _aswb_interact_icon (Utilities|Casting|CastToWB_InteractIcon (UserInterface|GetWidget (Variables|Default|GetWidget))))
      (Widget|SetVisibility (Variables|/Game/ForgettenRealms/HUD/WB_InteractIcon.WB_InteractIcon_C|GetHotkey _aswb_interact_icon) "Visible"))))

(event OnComponentEndOverlap(InteractPrompt)
  (params (OverlappedComponent :type Primitive%20Component%20Object%20Reference) (OtherActor :type Actor%20Object%20Reference) (OtherComp :type Primitive%20Component%20Object%20Reference) (OtherBodyIndex :type Integer))
  (Utilities|IsValid (Variables|Default|GetWidget)
    (:Is%20Valid
      (bind _aswb_interact_icon (Utilities|Casting|CastToWB_InteractIcon (UserInterface|GetWidget (Variables|Default|GetWidget))))
      (Widget|SetVisibility (Variables|/Game/ForgettenRealms/HUD/WB_InteractIcon.WB_InteractIcon_C|GetHotkey _aswb_interact_icon) "Hidden"))))

(event Custom|GainItems
  (bind _itemsinchest (Variables|Default|GetItemsInChest))
  (bind _returnvalue (Utilities|Array|Length _itemsinchest))
  (bind _returnvalue_2 (Math|Random|RandomInteger _returnvalue))
  (bind _output (Utilities|Array|Get(acopy) _itemsinchest _returnvalue_2))
  (bind _returnvalue_3 (UserInterface|CreateWidget "/Game/ForgettenRealms/HUD/WB_Item.WB_Item_C" 0 0))
  (bind _output_get (Variables|Default|SetItemWidgetREF _returnvalue_3))
  (UserInterface|Viewport|AddtoViewport _output_get 0)
  (if (Variables|Default|GetHasBomb?)
    (Default|GetItem (Variables|Default|GetItemWidgetREF) (Variables|Default|GetBomb))
    (bind _asbp_wukong_player (Utilities|Casting|CastToBP_WukongPlayer (Variables|Default|GetCharREF)))
    (Variables|/Game/ForgettenRealms/Player/BP_WukongPlayer.BP_WukongPlayer_C|SetHasBomb? _asbp_wukong_player true)
    (else
      (Default|GetItem (Variables|Default|GetItemWidgetREF) (Utilities|Struct|MakeSTRUCT_Item (.name _output) (.icon _output) (Math|Random|RandomInteger 5)) _returnvalue_2))))

(event EventInteract
  (if (not (or (Variables|Default|GetAnimating?) (Variables|Default|GetOpen?)))
    (Components|DestroyComponent (Variables|Default|GetWidget))
    (Variables|Default|SetAnimating? true)
    (bind _asbp_wukong_player (Utilities|Casting|CastToBP_WukongPlayer (Variables|Default|GetCharREF)))
    (bind _speed (Timeline|MovePlayerToChest PlayFromStart)
      (:Update
        (Transformation|SetActorLocation _asbp_wukong_player (Math|Vector|MakeVector (.x (Math|Vector|Lerp(Vector) (Transformation|GetActorLocation _asbp_wukong_player) (Transformation|GetWorldLocation (Variables|Default|GetOpenLocation)) _speed)) (.y (Math|Vector|Lerp(Vector) (Transformation|GetActorLocation _asbp_wukong_player) (Transformation|GetWorldLocation (Variables|Default|GetOpenLocation)) _speed)) (.Z (Math|Vector|BreakVector (Transformation|GetActorLocation _asbp_wukong_player)))) false false)
        (Transformation|SetActorRotation _asbp_wukong_player (Math|Rotator|MakeRotator 0.0 0.0 (.yaw (Math|Rotator|Lerp(Rotator) (Math|Rotator|MakeRotator (.roll (Transformation|GetActorRotation _asbp_wukong_player)) (.pitch (Transformation|GetActorRotation _asbp_wukong_player)) (.yaw (Transformation|GetActorRotation _asbp_wukong_player))) (Math|Rotator|MakeRotator (.roll (Transformation|GetActorRotation _asbp_wukong_player)) (.pitch (Transformation|GetActorRotation _asbp_wukong_player)) (.yaw (Math|Rotator|FindLookatRotation (Transformation|GetActorLocation _asbp_wukong_player) (Transformation|GetActorLocation)))) _speed)))))
      (:Finished
        (Default|HideStaff _asbp_wukong_player)
        (Input|DisableInput _asbp_wukong_player (Game|GetPlayerController 0))
        (Animation|Montage|PlayMontage (Variables|/Script/Engine.Character|GetMesh _asbp_wukong_player) "/Game/ForgettenRealms/Player/Wukong/Animation/RetargettedAnim/AM_OpenChest.AM_OpenChest" 2.75 0.5
          (:then
            (Audio|PlaySoundatLocation "/Game/ForgettenRealms/FX/SoundFX/Interactables/ChestOpen.ChestOpen" (Transformation|GetActorLocation) "0, 0, 0" 0.45 0.4 0.0 0 0 0 0)
            (Components|Animation|PlayAnimation (Variables|Default|GetChestOpenAnimation) "/Game/ForgettenRealms/StaticMeshes/Chest/ChestOpenAnimation_Anim.ChestOpenAnimation_Anim" false)
            (Variables|Default|SetOpen? true)
            (Utilities|FlowControl|Delay 1.25)
            (Variables|Default|SetAnimating? false))
          (:OnCompleted
            (Default|ShowStaff _asbp_wukong_player :!label _label)
            (Input|EnableInput _asbp_wukong_player (Game|GetPlayerController 0))
            (CallFunction|GainItems))
          (:OnInterrupted
            (goto _label)))))))

(event EventBeginPlay
  (Utilities|IsValid (Variables|Default|GetWidget)
    (:Is%20Valid
      (bind _aswb_interact_icon (Utilities|Casting|CastToWB_InteractIcon (UserInterface|GetWidget (Variables|Default|GetWidget))))
      (Variables|/Game/ForgettenRealms/HUD/WB_InteractIcon.WB_InteractIcon_C|SetInteractText _aswb_interact_icon (Variables|Default|GetInteractText))
      (Variables|Default|SetCharREF (Game|Player|GetPlayerPawn 0)))))

(fn ConstructionScript)