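; BP_Interactable is an interactable actor that shows a proximity prompt to the player through a WB_InteractIcon widget.
; On BeginPlay it hides the widget and passes InteractText into it.
; The outer VisiblePrompt overlap reveals the widget only for exact BP_WukongPlayer, while ActivationBox toggles the hotkey and text for any actor.
; Exits from either volume are unfiltered, and no interaction input is handled here.
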(event OnComponentBeginOverlap(VisiblePrompt)
  (params (OverlappedComponent :type Primitive%20Component%20Object%20Reference) (OtherActor :type Actor%20Object%20Reference) (OtherComp :type Primitive%20Component%20Object%20Reference) (OtherBodyIndex :type Integer) (bFromSweep :type Boolean) (SweepResult :type Hit%20Result%20Structure%20%28by%20ref%29))
  (bind _widget (Variables|Default|GetWidget))
  (Utilities|IsValid (Variables|Default|GetWidget)
    (:Is%20Valid
      (if (== (Utilities|GetClass OtherActor) "/Game/ForgettenRealms/Player/BP_WukongPlayer.BP_WukongPlayer_C")
        (Rendering|SetVisibility _widget true true)
        (Class|WidgetComponent|SetTickMode _widget "Enabled")))))

(event OnComponentEndOverlap(VisiblePrompt)
  (params (OverlappedComponent :type Primitive%20Component%20Object%20Reference) (OtherActor :type Actor%20Object%20Reference) (OtherComp :type Primitive%20Component%20Object%20Reference) (OtherBodyIndex :type Integer))
  (bind _widget (Variables|Default|GetWidget))
  (Utilities|IsValid (Variables|Default|GetWidget)
    (:Is%20Valid
      (Rendering|SetVisibility _widget false true)
      (Class|WidgetComponent|SetTickMode _widget "Automatic"))))

(event OnComponentBeginOverlap(ActivationBox)
  (params (OverlappedComponent :type Primitive%20Component%20Object%20Reference) (OtherActor :type Actor%20Object%20Reference) (OtherComp :type Primitive%20Component%20Object%20Reference) (OtherBodyIndex :type Integer) (bFromSweep :type Boolean) (SweepResult :type Hit%20Result%20Structure%20%28by%20ref%29))
  (bind _aswb_interact_icon (Utilities|Casting|CastToWB_InteractIcon (UserInterface|GetWidget (Variables|Default|GetWidget))))
  (Widget|SetVisibility (Variables|/Game/ForgettenRealms/HUD/WB_InteractIcon.WB_InteractIcon_C|GetHotkey _aswb_interact_icon) "Visible"))

(event OnComponentEndOverlap(ActivationBox)
  (params (OverlappedComponent :type Primitive%20Component%20Object%20Reference) (OtherActor :type Actor%20Object%20Reference) (OtherComp :type Primitive%20Component%20Object%20Reference) (OtherBodyIndex :type Integer))
  (bind _aswb_interact_icon (Utilities|Casting|CastToWB_InteractIcon (UserInterface|GetWidget (Variables|Default|GetWidget))))
  (Widget|SetVisibility (Variables|/Game/ForgettenRealms/HUD/WB_InteractIcon.WB_InteractIcon_C|GetHotkey _aswb_interact_icon) "Hidden"))

(event EventBeginPlay
  (bind _widget (Variables|Default|GetWidget))
  (Utilities|IsValid (Variables|Default|GetWidget)
    (:Is%20Valid
      (Rendering|SetVisibility _widget false false)
      (Class|WidgetComponent|SetTickMode _widget "Automatic")
      (bind _aswb_interact_icon (Utilities|Casting|CastToWB_InteractIcon (UserInterface|GetWidget (Variables|Default|GetWidget))))
      (Variables|/Game/ForgettenRealms/HUD/WB_InteractIcon.WB_InteractIcon_C|SetInteractText _aswb_interact_icon (Variables|Default|GetInteractText)))))

(fn ConstructionScript)