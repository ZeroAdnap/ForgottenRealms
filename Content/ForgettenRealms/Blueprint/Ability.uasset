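; Ability actor that activates itself on BeginPlay and destroys itself after its Cooldown via lifespan.
; Activation requires the owner's BP_PlayerStat to report at least CostValue of CostStat; the cost is checked but not deducted here.
; When the check passes, it spawns every class in Effects at the IntendedTarget's transform, or at the Caster's if no valid target exists.
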(event Custom|Activate%20Ability
  (bind _intendedtarget (Variables|Targetting|GetIntendedTarget))
  (if (CallFunction|CanActivateAbility)
    (for _array_element (Variables|AbilityDetails|GetEffects)
      (Game|SpawnActorfromClass _array_element (Math|Transform|SelectTransform (Transformation|GetActorTransform _intendedtarget) (Transformation|GetActorTransform (Variables|Targetting|GetCaster)) (Utilities|IsValid _intendedtarget)) "Undefined" "MultiplyWithRoot" 0 0))))

(event EventBeginPlay
  (CallFunction|ActivateAbility)
  (Actor|SetLifeSpan (Variables|AbilityDetails|GetCooldown)))

(event Collision|EventActorBeginOverlap
  (params (OtherActor :type Actor%20Object%20Reference)))

(event EventTick
  (params (DeltaSeconds :type Float%20%28single-precision%29)))

(fn ConstructionScript)

(fn CanActivateAbility
  (bind _value (Default|QueryStat (Actor|GetComponentbyClass (Components|GetOwner) "/Game/ForgettenRealms/Blueprint/BP_PlayerStat.BP_PlayerStat_C") (Variables|AbilityDetails|GetCostStat)))
  (return (>= _value (Variables|AbilityDetails|GetCostValue))))