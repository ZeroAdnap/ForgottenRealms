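; Melee enemy child Blueprint for the Hands variant, handling its attack combo and hit reactions.
; INTAttacking enables the hitbox and plays one of two montages by ComboHitCount, locking movement until completion, then increments the count and signals attack done at two or more.
; Hitbox overlaps apply fixed damage and print a debug string.
; Damage received updates the health widget and pauses movement during a hit montage.
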(event OnComponentBeginOverlap(MeleeAttackBox)
  (params (OverlappedComponent :type Primitive%20Component%20Object%20Reference) (OtherActor :type Actor%20Object%20Reference) (OtherComp :type Primitive%20Component%20Object%20Reference) (OtherBodyIndex :type Integer) (bFromSweep :type Boolean) (SweepResult :type Hit%20Result%20Structure%20%28by%20ref%29))
  (Game|Damage|ApplyDamage OtherActor 1e+01 0 0)
  (Development|PrintString (Utilities|String|Append "combo hit is" (Utilities|String|ToString(Integer) (Variables|Default|GetCombo%20hit%20count)))))

(event ReceivingDamage(BPC_Enemy_Health)
  (bind _bpc_enemy_health (Variables|Default|GetBPC_Enemy_Health))
  ;[1 1 1] Damage
  (Default|SetHealth (Variables|Default|GetAs%20WB%20Health) (Variables|/Game/ForgettenRealms/Enemies/Blueprint/BPC_Enemy_Health.BPC_Enemy_Health_C|GetMax%20Health _bpc_enemy_health) (Variables|/Game/ForgettenRealms/Enemies/Blueprint/BPC_Enemy_Health.BPC_Enemy_Health_C|GetHealth _bpc_enemy_health))
  (Pawn|Components|CharacterMovement|DisableMovement (Variables|Character|GetCharacterMovement))
  (bind _returnvalue (Animation|PlayAnimMontage "/Game/ForgettenRealms/Enemies/Animation/Skeleton/Anim_Hit_Montage.Anim_Hit_Montage" 1.0 "None"))
  (Utilities|FlowControl|Delay _returnvalue)
  (Pawn|Components|CharacterMovement|SetMovementMode (Variables|Character|GetCharacterMovement) "MOVE_Walking" 0))

(event EventBeginPlay
  (|CallParentFunction) ; This node is disabled and will not be called.\nDrag off pins to build functionality.
)

(event Collision|EventActorBeginOverlap
  (params (OtherActor :type Actor%20Object%20Reference))
  (|CallParentFunction OtherActor) ; This node is disabled and will not be called.\nDrag off pins to build functionality.
)

(event EventINTAttacking
  (CallFunction|HitBoxon)
  (Animation|Montage|PlayMontage (Variables|Character|GetMesh) (Utilities|Select :Index (Variables|Default|GetCombo%20hit%20count) :Option%200 "/Game/ForgettenRealms/Enemies/Animation/Skeleton/Anim_Attack_1_Montage.Anim_Attack_1_Montage" :Option%201 "/Game/ForgettenRealms/Enemies/Animation/Skeleton/Anim_Attack_2_Montage.Anim_Attack_2_Montage")
    (:then
      (Pawn|Components|CharacterMovement|DisableMovement (Variables|Character|GetCharacterMovement)))
    (:OnCompleted
      (Pawn|Components|CharacterMovement|SetMovementMode (Variables|Character|GetCharacterMovement) "MOVE_Walking" 0)
      (CallFunction|HitBoxOff)
      (bind _result (Math|Integer|IncrementInt (Variables|Default|GetCombo%20hit%20count))
        (:%20%20
          (if (>= _result 2)
            (Class|BPIMinion|INTDoneAttack(Message) self)))))))

(fn ConstructionScript
  (|CallParentFunction))