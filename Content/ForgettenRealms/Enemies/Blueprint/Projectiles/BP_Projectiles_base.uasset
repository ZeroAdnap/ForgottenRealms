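; Base enemy projectile actor that flies forward and damages the Wukong player.
; Each tick it moves by an XOnly local offset without sweeping or delta-time scaling, and it destroys itself after a fixed lifetime.
; Its PlayerDamgeProjectiles event applies fixed damage if the passed actor is the BP_WukongPlayer found by class lookup, then destroys the projectile whatever the actor was.
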(event Custom|PlayerDamgeProjectiles
  (params (Other%20Actor :type Object%20Object%20Reference))
  (Utilities|FlowControl|Sequence
    (:then_0
      (bind _returnvalue (Actor|GetActorOfClass "/Game/ForgettenRealms/Player/BP_WukongPlayer.BP_WukongPlayer_C"))
      (if (== _returnvalue Other%20Actor)
        (Game|Damage|ApplyDamage _returnvalue 5e+01 0 0)))
    (:then_1
      (Actor|DestroyActor))))

(event EventTick
  (params (DeltaSeconds :type Float%20%28single-precision%29))
  (Transformation|AddActorLocalOffset (Variables|Default|GetX%20Only) false false))

(event EventBeginPlay
  (Utilities|FlowControl|Delay 1e+01)
  (Actor|DestroyActor))

(fn ConstructionScript)