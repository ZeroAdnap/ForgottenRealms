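; BP_Arrow is an enemy arrow projectile that plays a 2D whoosh sound when it spawns.
; When its capsule overlaps an actor, it plays an impact sound at the sweep impact point and passes that actor to PlayerDamgeProjectiles, which is defined outside this graph.
; A blocking hit on the capsule destroys the arrow, while an overlap does not destroy it in this graph.
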(event OnComponentBeginOverlap(Capsule)
  (params (OverlappedComponent :type Primitive%20Component%20Object%20Reference) (OtherActor :type Actor%20Object%20Reference) (OtherComp :type Primitive%20Component%20Object%20Reference) (OtherBodyIndex :type Integer) (bFromSweep :type Boolean) (SweepResult :type Hit%20Result%20Structure%20%28by%20ref%29))
  (Audio|PlaySoundatLocation "/Game/ForgettenRealms/Enemies/SFX/Arrow.Arrow" (.impactpoint SweepResult) "0, 0, 0" 0.75 1.2 0.0 0 0 0 0)
  (CallFunction|PlayerDamgeProjectiles OtherActor))

(event OnComponentHit(Capsule)
  (params (HitComponent :type Primitive%20Component%20Object%20Reference) (OtherActor :type Actor%20Object%20Reference) (OtherComp :type Primitive%20Component%20Object%20Reference) (NormalImpulse :type Vector :default "0, 0, 0") (Hit :type Hit%20Result%20Structure%20%28by%20ref%29))
  (Actor|DestroyActor))

(event EventBeginPlay
  (|CallParentFunction)
  (Audio|PlaySound2D "/Game/ForgettenRealms/Enemies/SFX/arrow-cutting-through-the-air-39540.arrow-cutting-through-the-air-39540" 1.0 1.0 0.0 0 0))

(event Collision|EventActorBeginOverlap
  (params (OtherActor :type Actor%20Object%20Reference)))

(event EventTick
  (params (DeltaSeconds :type Float%20%28single-precision%29))
  (|CallParentFunction DeltaSeconds) ; This node is disabled and will not be called.\nDrag off pins to build functionality.
)

(fn ConstructionScript
  (|CallParentFunction))