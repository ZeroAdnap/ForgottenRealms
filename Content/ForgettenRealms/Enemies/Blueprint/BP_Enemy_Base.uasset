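; Base enemy Blueprint handling health display, death, movement speed and montage combo attacks.
; BPC_Enemy_Health events update the widget, briefly halt movement on damage, and on death ragdoll the mesh, stop AI, award player XP and destroy the actor.
; Tick yaws the health bar toward the camera and clears zone blackboard keys when TooFarFromZone is true.
; Attacks pick montages by combo counter, disabling movement during playback.
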(event Death(BPC_Enemy_Health)
  ;[1 1 1] Death
  (Utilities|FlowControl|Sequence
    (:then_0
      (Rendering|SetVisibility (Variables|Default|GetWidget) false false)
      (Pawn|Components|CharacterMovement|DisableMovement (Variables|Character|GetCharacterMovement))
      (Collision|SetCollisionResponsetoChannel (Variables|Character|GetMesh) "ECC_GameTraceChannel3" "ECR_Overlap")
      (Physics|SetSimulatePhysics (Variables|Character|GetMesh) true)
      (AI|Logic|StopLogic (Variables|/Script/AIModule.AIController|GetBrainComponent (AI|GetAIController self)) "Dead"))
    (:then_1
      (Utilities|FlowControl|Delay 2.5)
      (Actor|DestroyActor))
    (:then_2
      (bind _asbp_wukong_player (Utilities|Casting|CastToBP_WukongPlayer (Game|Player|GetPlayerPawn 0)))
      (Default|IncreaseXP (Variables|/Game/ForgettenRealms/Player/BP_WukongPlayer.BP_WukongPlayer_C|GetBP_PlayerStat _asbp_wukong_player) (Variables|Default|GetAdded%20XP)))))

(event ReceivingDamage(BPC_Enemy_Health)
  (bind _bpc_enemy_health (Variables|Default|GetBPC_Enemy_Health))
  (Default|SetHealth (Variables|Default|GetAs%20WB%20Health) (Variables|/Game/ForgettenRealms/Enemies/Blueprint/Component/BPC_Enemy_Health.BPC_Enemy_Health_C|GetMax%20Health _bpc_enemy_health) (Variables|/Game/ForgettenRealms/Enemies/Blueprint/Component/BPC_Enemy_Health.BPC_Enemy_Health_C|GetHealth _bpc_enemy_health))
  (Pawn|Components|CharacterMovement|DisableMovement (Variables|Character|GetCharacterMovement))
  (Utilities|FlowControl|Delay 0.4)
  (Pawn|Components|CharacterMovement|SetMovementMode (Variables|Character|GetCharacterMovement) "MOVE_Walking" 0))

(event Custom|Attacking
  (params (Montages :type Array%20of%20Anim%20Montage%20Object%20References))
  (bind _charactermovement (Variables|Character|GetCharacterMovement))
  (Variables|Default|SetComboAmount (Utilities|Array|Length Montages))
  (Animation|Montage|PlayMontage (Variables|Character|GetMesh) (Utilities|Array|Get(acopy) Montages (Variables|Default|GetCombo%20hit%20count))
    (:then
      (Pawn|Components|CharacterMovement|DisableMovement _charactermovement)
      (bind _result (Math|Integer|IncrementInt (Variables|Default|GetCombo%20hit%20count) :!label _label)
        (:%20%20
          (if (> _result (Variables|Default|GetComboAmount))
            (Class|BPIEnemy|INTDoneAttack(Message) self)))))
    (:OnCompleted
      (Pawn|Components|CharacterMovement|SetMovementMode _charactermovement "MOVE_Walking" 0)
      (goto _label))
    (:OnInterrupted
      (Class|BPIEnemy|INTDoneAttack(Message) self)
      (Pawn|Components|CharacterMovement|SetMovementMode (Variables|Character|GetCharacterMovement) "MOVE_Walking" 0))))

(event EventINTChangingSpeed
  (params (Speed :type Float%20%28double-precision%29))
  (Variables|/Script/Engine.CharacterMovementComponent|SetMaxWalkSpeed (Variables|Character|GetCharacterMovement) Speed)
  (Variables|Default|SetSpeedChanged true))

(event EventTick
  (params (DeltaSeconds :type Float%20%28single-precision%29))
  (bind _self self)
  (bind _returnvalue (AI|GetAIController _self))
  (bind _returnvalue_2 (AI|GetBlackboard _returnvalue))
  (Utilities|HealthBarLookatPlayer
    (:Output
      (if (Utilities|TooFarfromZone?)
        (AI|Components|Blackboard|SetValueasBool _returnvalue_2 (Utilities|Name|MakeLiteralName "inZone") false)
        (AI|Components|Blackboard|SetValueasBool _returnvalue_2 (Utilities|Name|MakeLiteralName "lastLocationVisited") false)))))

(event EventBeginPlay
  (bind _bpc_enemy_health (Variables|Default|GetBPC_Enemy_Health))
  (bind _aswb_health (Utilities|Casting|CastToWB_Health (UserInterface|GetWidget (Variables|Default|GetWidget))))
  (bind _output_get (Variables|Default|SetAs%20WB%20Health _aswb_health))
  (Default|SetHealth _output_get (Variables|/Game/ForgettenRealms/Enemies/Blueprint/Component/BPC_Enemy_Health.BPC_Enemy_Health_C|GetMax%20Health _bpc_enemy_health) (Variables|/Game/ForgettenRealms/Enemies/Blueprint/Component/BPC_Enemy_Health.BPC_Enemy_Health_C|GetHealth _bpc_enemy_health)))

(event EventINTDoneAttack
  (Variables|Default|SetCombo%20hit%20count 0))

(event EventChangeSpeedRun
  (Variables|/Script/Engine.CharacterMovementComponent|SetMaxWalkSpeed (Variables|Character|GetCharacterMovement) 4.5e+02))

(event EventChangeSpeedIdle
  (Variables|/Script/Engine.CharacterMovementComponent|SetMaxWalkSpeed (Variables|Character|GetCharacterMovement) 2e+02))

(fn ConstructionScript)