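; Mountain dragon boss built on a parent enemy class, turning each tick and fighting the Wukong player with claw, bite and fireball attacks.
; Interface events trigger the attacks, with toggleable hitboxes for melee damage and fireballs spawned aimed at the player.
; Hits at 30% health or below double damage once and start a timed flight phase through Blackboard state and takeoff/landing flags.
; The health component also triggers a random death montage.
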(event DeathAnim(BPC_Enemy_Health)
  ;[1 1 1] Death Anim
  (Utilities|FlowControl|DoOnce false
    (:Completed
      (Animation|Montage|PlayMontage 0 (Utilities|Select :Index (Math|Random|RandomIntegerinRange 0 1) :Option%200 "/Game/ForgettenRealms/Enemies/Animation/Dragon/ANIM_MOUNTAIN_DRAGON_death_Montage.ANIM_MOUNTAIN_DRAGON_death_Montage" :Option%201 "/Game/ForgettenRealms/Enemies/Animation/Dragon/ANIM_MOUNTAIN_DRAGON_deathHitTheGround_Montage.ANIM_MOUNTAIN_DRAGON_deathHitTheGround_Montage")))))

(event HitAnim(BPC_Enemy_Health)
  (bind _bpc_enemy_health (Variables|Default|GetBPC_Enemy_Health))
  ;[1 1 1] change mode to fly
  (if (<= (Variables|/Game/ForgettenRealms/Enemies/Blueprint/Component/BPC_Enemy_Health.BPC_Enemy_Health_C|GetHealth _bpc_enemy_health) (* (Variables|/Game/ForgettenRealms/Enemies/Blueprint/Component/BPC_Enemy_Health.BPC_Enemy_Health_C|GetMax%20Health _bpc_enemy_health) 0.3))
    (Utilities|FlowControl|Sequence
      (:then_0
        (Utilities|FlowControl|DoOnce false
          (:Completed
            (Variables|Default|SetBase%20Damage (* (Variables|Default|GetBase%20Damage) 2.0)))))
      (:then_1
        (Variables|Default|SetTakeOff? true)
        (Utilities|FlowControl|Delay 1.0)
        (Variables|Default|SetTakeOff? false))
      (:then_2
        (Utilities|ChangeMode "NewEnumerator4")
        (Utilities|FlowControl|Delay 15.0)
        (Variables|Default|SetLanding? true)
        (Utilities|ChangeMode "NewEnumerator1")
        (Utilities|FlowControl|Delay 0.5)
        (Variables|Default|SetLanding? false)))))

(event OnComponentBeginOverlap(BodyBox1)
  (params (OverlappedComponent :type Primitive%20Component%20Object%20Reference) (OtherActor :type Actor%20Object%20Reference) (OtherComp :type Primitive%20Component%20Object%20Reference) (OtherBodyIndex :type Integer) (bFromSweep :type Boolean) (SweepResult :type Hit%20Result%20Structure%20%28by%20ref%29))
  (bind _returnvalue (Actor|GetActorOfClass "/Game/ForgettenRealms/Player/BP_WukongPlayer.BP_WukongPlayer_C"))
  (if (== OverlappedComponent (Variables|/Game/ForgettenRealms/Player/BP_WukongPlayer.BP_WukongPlayer_C|GetAttackBox _returnvalue))
    (Game|Damage|ApplyDamage self (Variables|/Game/ForgettenRealms/Player/BP_WukongPlayer.BP_WukongPlayer_C|GetDamageApplied _returnvalue) 0 0)))

(event OnComponentBeginOverlap(Mesh)
  (params (OverlappedComponent :type Primitive%20Component%20Object%20Reference) (OtherActor :type Actor%20Object%20Reference) (OtherComp :type Primitive%20Component%20Object%20Reference) (OtherBodyIndex :type Integer) (bFromSweep :type Boolean) (SweepResult :type Hit%20Result%20Structure%20%28by%20ref%29))
  (bind _returnvalue (Actor|GetActorOfClass "/Game/ForgettenRealms/Player/BP_WukongPlayer.BP_WukongPlayer_C"))
  (if (== (stale OnComponentBeginOverlap(BodyBox1) OverlappedComponent) (Variables|/Game/ForgettenRealms/Player/BP_WukongPlayer.BP_WukongPlayer_C|GetAttackBox _returnvalue))
    (Game|Damage|ApplyDamage self (Variables|/Game/ForgettenRealms/Player/BP_WukongPlayer.BP_WukongPlayer_C|GetDamageApplied _returnvalue) 0 0)))

(event OnComponentBeginOverlap(LClawAttackBox)
  (params (OverlappedComponent :type Primitive%20Component%20Object%20Reference) (OtherActor :type Actor%20Object%20Reference) (OtherComp :type Primitive%20Component%20Object%20Reference) (OtherBodyIndex :type Integer) (bFromSweep :type Boolean) (SweepResult :type Hit%20Result%20Structure%20%28by%20ref%29))
  ;[1 1 1] Claw Attack
  (Game|Damage|ApplyDamage OtherActor (Variables|Default|GetBase%20Damage) 0 0))

(event OnComponentBeginOverlap(RClawAttackBox)
  (params (OverlappedComponent :type Primitive%20Component%20Object%20Reference) (OtherActor :type Actor%20Object%20Reference) (OtherComp :type Primitive%20Component%20Object%20Reference) (OtherBodyIndex :type Integer) (bFromSweep :type Boolean) (SweepResult :type Hit%20Result%20Structure%20%28by%20ref%29))
  ;[1 1 1] Claw Attack
  (Game|Damage|ApplyDamage OtherActor (Variables|Default|GetBase%20Damage) 0 0))

(event OnComponentBeginOverlap(BiteAttackBox)
  (params (OverlappedComponent :type Primitive%20Component%20Object%20Reference) (OtherActor :type Actor%20Object%20Reference) (OtherComp :type Primitive%20Component%20Object%20Reference) (OtherBodyIndex :type Integer) (bFromSweep :type Boolean) (SweepResult :type Hit%20Result%20Structure%20%28by%20ref%29))
  ;[1 1 1] BiteAttack
  (Game|Damage|ApplyDamage OtherActor (Variables|Default|GetBase%20Damage) 0 0))

(event Custom|BiteHitBox
  (params (On/Off :type Boolean))
  (bind _biteattackbox (Variables|Default|GetBiteAttackBox))
  ;[1 1 1] BiteAttack
  (if On/Off
    (Collision|SetCollisionEnabled _biteattackbox "QueryOnly")
    (else
      (Collision|SetCollisionEnabled _biteattackbox "NoCollision"))))

(event Custom|RClawHitBox
  (params (On/Off :type Boolean))
  (bind _rclawattackbox (Variables|Default|GetRClawAttackBox))
  ;[1 1 1] Claw Attack
  (if On/Off
    (Collision|SetCollisionEnabled _rclawattackbox "QueryOnly")
    (else
      (Collision|SetCollisionEnabled _rclawattackbox "NoCollision"))))

(event Custom|LClawHitBox
  (params (On/Off :type Boolean))
  (bind _lclawattackbox (Variables|Default|GetLClawAttackBox))
  ;[1 1 1] Claw Attack
  (if On/Off
    (Collision|SetCollisionEnabled _lclawattackbox "QueryOnly")
    (else
      (Collision|SetCollisionEnabled _lclawattackbox "NoCollision"))))

(event EventBeginPlay
  ;[1 1 1] BeginPlay
  (|CallParentFunction)
  (Variables|Default|SetDeathDuration 15.0))

(event EventINTClawAttack
  ;[1 1 1] interface attacks
  (CallFunction|Attacks (Variables|Default|GetClaw%20Attack)))

(event EventTick
  (params (DeltaSeconds :type Float%20%28single-precision%29))
  ;[1 1 1] Look at rotation
  (|CallParentFunction DeltaSeconds)
  (CallFunction|CheckDistance self)
  (CallFunction|RotateActorinDirection))

(event EventINTBiteAttack
  ;[1 1 1] interface attacks
  (CallFunction|Attacks (Variables|Default|GetBite%20Attack)))

(event EventINTLookat
  ;[1 1 1] Look at rotation
)

(event EventINTRangeAttack
  ;[1 1 1] interface attacks
  (CallFunction|Attacks (Variables|Default|GetRange%20Attack)))

(event EventINTSpawnRangeAttack
  (bind _fireball_spawn_location (Variables|Default|Getfireball%20spawn%20location))
  (bind _returnvalue (Transformation|GetWorldTransform _fireball_spawn_location))
  ;[1 1 1] interface attacks
  (CallFunction|SpawnRangeAttack "/Game/ForgettenRealms/Enemies/Blueprint/Projectiles/BP_Fireball.BP_Fireball_C" (.location _returnvalue) (Math|Rotator|FindLookatRotation (.location _returnvalue) (Transformation|GetActorLocation (Variables|Default|GetAs%20BP%20Wukong%20Player))) "7.000000,7.000000,7.000000")
  (bind _result (Math|Integer|IncrementInt (Variables|Default|GetrangeAttackAmount))
    (:%20%20
      (if (== _result 2)
        (Utilities|FlowControl|Delay 8.0)
        (Variables|Default|SetrangeAttackAmount 0)))))

(fn ConstructionScript
  (|CallParentFunction))