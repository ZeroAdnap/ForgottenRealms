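; BP_Enemy_Melee is a melee enemy character that performs montage-driven combo attacks.
; Attacking plays the montage at the current combo index, disables movement, increments the hit count and calls INTDoneAttackMessage once it exceeds the combo amount.
; Montage completion or interruption restores walking, with interruption also sending the done message.
; Separate events switch the MeleeAttackBox collision between query-only and off to control the hit window.
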(event Custom|MeleeHitBoxOff
  (Collision|SetCollisionEnabled (Variables|Default|GetMeleeAttackBox) "NoCollision"))

(event Custom|MeleeHitBoxOn
  (Collision|SetCollisionEnabled (Variables|Default|GetMeleeAttackBox) "QueryOnly"))

(event Custom|Attacking
  (params (Montages :type Array%20of%20Anim%20Montage%20Object%20References))
  (bind _charactermovement (Variables|Character|GetCharacterMovement))
  (Animation|Montage|PlayMontage (Variables|Character|GetMesh) (Utilities|Array|Get(acopy) Montages (Variables|Default|GetCombo%20hit%20count))
    (:then
      (Pawn|Components|CharacterMovement|DisableMovement _charactermovement)
      (bind _result (Math|Integer|IncrementInt (Variables|Default|GetCombo%20hit%20count))
        (:%20%20
          (if (> _result (Variables|Default|GetComboAmount))
            (Class|BPIMinion|INTDoneAttack(Message) self)))))
    (:OnCompleted
      (Pawn|Components|CharacterMovement|SetMovementMode _charactermovement "MOVE_Walking" 0))
    (:OnInterrupted
      (Class|BPIMinion|INTDoneAttack(Message) self)
      (Pawn|Components|CharacterMovement|SetMovementMode (Variables|Character|GetCharacterMovement) "MOVE_Walking" 0))))

(event EventBeginPlay
  (|CallParentFunction) ; This node is disabled and will not be called.\nDrag off pins to build functionality.
)

(event Collision|EventActorBeginOverlap
  (params (OtherActor :type Actor%20Object%20Reference)))

(event EventTick
  (params (DeltaSeconds :type Float%20%28single-precision%29))
  (|CallParentFunction DeltaSeconds) ; This node is disabled and will not be called.\nDrag off pins to build functionality.
)

(fn ConstructionScript
  (|CallParentFunction))