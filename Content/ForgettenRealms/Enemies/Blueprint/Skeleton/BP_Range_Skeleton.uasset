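; Ranged skeleton enemy, a child Blueprint that attacks the player with bow and arrows.
; BeginPlay writes its enemy type to the AI controller's Blackboard, and Tick runs a distance check.
; Interface-style events play the attack and bow animations, then spawn an arrow rotated toward the player.
; Death from the health component plays a montage and destroys the actor after its duration; footsteps play a sound.
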(event DeathAnim(BPC_Enemy_Health)
  (bind _returnvalue (Animation|PlayAnimMontage (Variables|Default|GetDeathAnimation) 1.0 "None"))
  (Utilities|FlowControl|Delay _returnvalue)
  (Actor|DestroyActor))

(event Custom|SetType
  (AI|Components|Blackboard|SetValueasEnum (Variables|/Script/AIModule.AIController|GetBlackboard (AI|GetAIController self)) (Utilities|Name|MakeLiteralName "EnemyType") (Utilities|Enum|LiteralenumE_EnemyType "NewEnumerator2")))

(event EventBeginPlay
  (|CallParentFunction)
  (CallFunction|SetType))

(event Collision|EventActorBeginOverlap
  (params (OtherActor :type Actor%20Object%20Reference))
  (|CallParentFunction OtherActor) ; This node is disabled and will not be called.\nDrag off pins to build functionality.
)

(event EventTick
  (params (DeltaSeconds :type Float%20%28single-precision%29))
  (|CallParentFunction DeltaSeconds)
  (CallFunction|CheckDistance self))

(event EventFootstep
  (Audio|PlaySoundatLocation "/Game/ForgettenRealms/Enemies/SFX/SkeletonStep_Cue.SkeletonStep_Cue" (Transformation|GetActorLocation) "0, 0, 0" 1.0 1.0 0.0 0 0 0 0))

(event EventINTRangeAttack
  (CallFunction|Attacks (Variables|Default|GetRange%20Attack))
  (Components|Animation|PlayAnimation (Variables|Default|GetBow) "/Game/ForgettenRealms/Enemies/Animation/Skeleton/Bow/Anim_Bow_Attack.Anim_Bow_Attack" false))

(event EventINTSpawnRangeAttack
  (bind _scene (Variables|Default|GetScene))
  (bind _returnvalue (Transformation|GetWorldTransform _scene))
  (CallFunction|SpawnRangeAttack "/Game/ForgettenRealms/Enemies/Blueprint/Projectiles/BP_Arrow.BP_Arrow_C" (.location _returnvalue) (Math|Rotator|FindLookatRotation (.location _returnvalue) (Transformation|GetActorLocation (Variables|Default|GetAs%20BP%20Wukong%20Player))) "1.000000,1.000000,1.000000"))

(fn ConstructionScript
  (|CallParentFunction))