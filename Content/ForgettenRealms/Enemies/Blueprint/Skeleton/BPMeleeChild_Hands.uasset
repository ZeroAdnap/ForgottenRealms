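; BPMeleeChild_Hands is a melee skeleton enemy child Blueprint that supplies its attack, hit and death behavior.
; The attack interface event passes MeleeAttackAnim to Attacks, and MeleeAttackBox overlaps apply BaseDamage to the other actor.
; Hits from the health component play a montage, then restore walking after its duration; construction assigns the death montage.
; An older two-montage combo chain with movement locking remains disconnected and never runs.
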(event OnComponentBeginOverlap(MeleeAttackBox)
  (params (OverlappedComponent :type Primitive%20Component%20Object%20Reference) (OtherActor :type Actor%20Object%20Reference) (OtherComp :type Primitive%20Component%20Object%20Reference) (OtherBodyIndex :type Integer) (bFromSweep :type Boolean) (SweepResult :type Hit%20Result%20Structure%20%28by%20ref%29))
  (Game|Damage|ApplyDamage OtherActor (Variables|Default|GetBase%20Damage) 0 0))

(event HitAnim(BPC_Enemy_Health)
  ;[1 1 1] Damage
  (bind _returnvalue (Animation|PlayAnimMontage "/Game/ForgettenRealms/Enemies/Animation/Skeleton/Hand/Anim_Hit_Montage.Anim_Hit_Montage" 1.0 "None"))
  (Utilities|FlowControl|Delay _returnvalue)
  (Pawn|Components|CharacterMovement|SetMovementMode (Variables|Character|GetCharacterMovement) "MOVE_Walking" 0))

(event EventBeginPlay
  (|CallParentFunction) ; This node is disabled and will not be called.\nDrag off pins to build functionality.
)

(event Collision|EventActorBeginOverlap
  (params (OtherActor :type Actor%20Object%20Reference))
  (|CallParentFunction OtherActor) ; This node is disabled and will not be called.\nDrag off pins to build functionality.
)

(event EventINTAttacking
  (CallFunction|Attacks (Variables|Default|GetMelee%20Attack%20Anim)))

(fn ConstructionScript
  (|CallParentFunction)
  (Variables|Default|SetDeathAnimation "/Game/ForgettenRealms/Enemies/Animation/Skeleton/Hand/Anim_Death_Montage.Anim_Death_Montage"))