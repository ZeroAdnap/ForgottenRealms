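; BP_OriginalPoint marks a spherical allowed area that tracks when enemies leave it.
; When a component tagged Enemy stops overlapping AllowedArea, the owning actor's AI blackboard gets its allowedZone and lastLocationVisited flags cleared.
; The Blueprint only writes these flags on exit and never sets them back on entry.
; BeginPlay draws a temporary debug sphere at the root using the area's radius.
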(event OnComponentEndOverlap(allowedArea)
  (params (OverlappedComponent :type Primitive%20Component%20Object%20Reference) (OtherActor :type Actor%20Object%20Reference) (OtherComp :type Primitive%20Component%20Object%20Reference) (OtherBodyIndex :type Integer))
  (bind _returnvalue (AI|GetAIController OtherActor))
  (bind _returnvalue_2 (AI|GetBlackboard _returnvalue))
  (if (Components|ComponentHasTag OtherComp "Enemy")
    (AI|Components|Blackboard|SetValueasBool _returnvalue_2 (Utilities|Name|MakeLiteralName "allowedZone") false)
    (AI|Components|Blackboard|SetValueasBool _returnvalue_2 (Utilities|Name|MakeLiteralName "lastLocationVisited") false)))

(event EventBeginPlay
  (Rendering|Debug|DrawDebugSphere (Transformation|GetWorldLocation (Variables|Default|GetDefaultSceneRoot)) (Variables|/Script/Engine.SphereComponent|GetSphereRadius (Variables|Default|GetallowedArea)) 12 "(R=1.000000,G=0.000000,B=0.035882,A=1.000000)" 1e+02))

(fn ConstructionScript)