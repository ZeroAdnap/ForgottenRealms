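; Arena enemy spawner that runs up to five waves, opened by StartWaves with a battle horn and short delay.
; SpawnWave spawns the wave's EnemyWaves classes at random navigable points around itself, tagging each as an arena enemy with this spawner as origin.
; Tick watches EnemyCount and, when it empties, uses a DoOnce re-armed during spawning to launch the next wave.
; EndWaves is an empty stub.
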(event Custom|SpawnWave
  (for _array_element (Utilities|Struct|BreakSTRUCT_EnemyWave (.Value (Utilities|Map|Find (Variables|Default|GetEnemyWaves) (Variables|Default|GetWaveNumber))))
    (bind _randomlocation (Class|NavigationSystemV1|GetRandomLocationinNavigableRadius (Transformation|GetActorLocation) (Variables|Default|GetSpawnDistance) 0 0))
    (bind _returnvalue (Game|SpawnActorfromClass _array_element (Math|Transform|MakeTransform _randomlocation (Math|Rotator|MakeRotator 0.0 0.0 0.0) "1.000000,1.000000,1.000000") "AdjustIfPossibleButAlwaysSpawn" "MultiplyWithRoot" 0 0))
    (Utilities|Array|Add (Variables|Default|GetSpawnedEnemies) _returnvalue)
    (Class|Actor|AddActorWorldRotation _returnvalue (Math|Rotator|MakeRotator 0.0 0.0 (Utilities|GetRotationtoPlayer _returnvalue)))
    (bind _asbp_enemy_base (Utilities|Casting|CastToBP_Enemy_Base _returnvalue))
    (Variables|/Game/ForgettenRealms/Enemies/Blueprint/BaseEnemies/BP_Enemy_Base.BP_Enemy_Base_C|SetArenaEnemy? _asbp_enemy_base true)
    (Variables|/Game/ForgettenRealms/Enemies/Blueprint/BaseEnemies/BP_Enemy_Base.BP_Enemy_Base_C|SetOrigin _asbp_enemy_base self)
    (Math|Integer|IncrementInt (Variables|Default|GetEnemyCount)
      (:%20%20
        (CallFunction|ResetWave)))))

(event Custom|StartWaves
  (Audio|PlaySoundatLocation "/Game/ForgettenRealms/FX/SoundFX/BattleHorn2.BattleHorn2" (Transformation|GetActorLocation) "0, 0, 0" 0.45 1.0 0.1 0 0 0 0)
  (Utilities|FlowControl|Delay 4.0)
  (Math|Integer|IncrementInt (Variables|Default|GetWaveNumber)
    (:%20%20
      (CallFunction|SpawnWave)
      (Variables|Default|SetActive? true))))

(event Custom|EndWaves
  (if (>= (Variables|Default|GetWaveNumber) 5)
    _))

(event Custom|ResetWave
  (Utilities|FlowControl|DoOnce false) ; enters at Reset
)

(event EventBeginPlay)

(event EventTick
  (params (DeltaSeconds :type Float%20%28single-precision%29))
  (if (Variables|Default|GetActive?)
    (if (<= (Variables|Default|GetEnemyCount) 0)
      (if (< (Variables|Default|GetWaveNumber) 5)
        (Utilities|FlowControl|DoOnce false
          (:Completed
            (Math|Integer|IncrementInt (Variables|Default|GetWaveNumber)
              (:%20%20
                (Audio|PlaySoundatLocation "/Game/ForgettenRealms/FX/SoundFX/BattleHorn2.BattleHorn2" (Transformation|GetActorLocation) "0, 0, 0" 0.45 1.0 0.1 0 0 0 0)
                (Utilities|FlowControl|Delay 4.0)
                (CallFunction|SpawnWave)))))
        (else
          (CallFunction|EndWaves))))))

(fn ConstructionScript)