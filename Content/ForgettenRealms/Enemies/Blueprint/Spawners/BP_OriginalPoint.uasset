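; Enemy spawn point that fills the navmesh around itself with a chosen enemy type up to a cap.
; Each enemy receives this point as its Origin; centaurs also get a wider origin distance and two uncounted minions.
; Spawning recurses on BeginPlay and on respawn until the cap is reached.
; BP_WukongPlayer entering the cull sphere blocks respawning, while any overlap end re-enables it and starts a delayed refill timer.
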(event OnComponentBeginOverlap(CullRespawnRadius)
  (params (OverlappedComponent :type Primitive%20Component%20Object%20Reference) (OtherActor :type Actor%20Object%20Reference) (OtherComp :type Primitive%20Component%20Object%20Reference) (OtherBodyIndex :type Integer) (bFromSweep :type Boolean) (SweepResult :type Hit%20Result%20Structure%20%28by%20ref%29))
  (if (== (Utilities|GetClass OtherActor) "/Game/ForgettenRealms/Player/BP_WukongPlayer.BP_WukongPlayer_C")
    (Variables|Default|SetCanRespawn? false)
    (Utilities|Time|ClearTimerbyFunctionName 0 "RespawnEnemies")))

(event OnComponentEndOverlap(CullRespawnRadius)
  (params (OverlappedComponent :type Primitive%20Component%20Object%20Reference) (OtherActor :type Actor%20Object%20Reference) (OtherComp :type Primitive%20Component%20Object%20Reference) (OtherBodyIndex :type Integer))
  (Variables|Default|SetCanRespawn? true)
  (bind _returnvalue (Utilities|Time|SetTimerbyFunctionName 0 "RespawnEnemies" 9e+01))
  (Variables|Default|SetTimer _returnvalue))

(event Custom|FirstSpawn
  (if (< (Variables|Default|GetCurrentSpawnCount) (Variables|Default|GetMaxSpawnCount))
    (bind _randomlocation (Class|NavigationSystemV1|GetRandomLocationinNavigableRadius (Transformation|GetActorLocation) (Variables|Default|GetRespawnRadius) 0 0))
    (bind _returnvalue (Game|SpawnActorfromClass (Variables|Default|GetSpawnerActorType) (Math|Transform|MakeTransform _randomlocation "0, 0, 0" "1.000000,1.000000,1.000000") "AdjustIfPossibleButAlwaysSpawn" "MultiplyWithRoot" 0 0))
    (bind _asbp_enemy_base (Utilities|Casting|CastToBP_Enemy_Base _returnvalue))
    (Variables|/Game/ForgettenRealms/Enemies/Blueprint/BaseEnemies/BP_Enemy_Base.BP_Enemy_Base_C|SetOrigin _asbp_enemy_base self)
    (Math|Integer|IncrementInt (Variables|Default|GetCurrentSpawnCount)
      (:%20%20
        (if (== (Variables|Default|GetSpawnerActorType) "/Game/ForgettenRealms/Enemies/Blueprint/Centaur/BP_Enemy_Melee_Centaur.BP_Enemy_Melee_Centaur_C")
          (Variables|/Game/ForgettenRealms/Enemies/Blueprint/BaseEnemies/BP_Enemy_Base.BP_Enemy_Base_C|SetOriginDistance _asbp_enemy_base 5e+03)
          ;[1 1 1] Spawn 2 centaurs around the original one
          (CallFunction|SpawnMinions (Transformation|GetActorLocation _returnvalue))
          (CallFunction|SpawnMinions (Transformation|GetActorLocation _returnvalue)))
        (if (Variables|Default|GetFirstSpawn?)
          ;[1 1 1] Continue to spawn the first wave (On begin play)
          (CallFunction|FirstSpawn)
          (else
            ;[1 1 1] Respawn Enemies as Normal
            (CallFunction|RespawnEnemies)))))
    (else
      (Variables|Default|SetCanRespawn? false)
      (Variables|Default|SetFirstSpawn? false))))

(event Custom|RespawnEnemies
  (if (Variables|Default|GetCanRespawn?)
    (if (< (Variables|Default|GetCurrentSpawnCount) (Variables|Default|GetMaxSpawnCount))
      (bind _randomlocation (Class|NavigationSystemV1|GetRandomLocationinNavigableRadius (Transformation|GetActorLocation) (Variables|Default|GetRespawnRadius) 0 0))
      (bind _returnvalue (Game|SpawnActorfromClass (Variables|Default|GetSpawnerActorType) (Math|Transform|MakeTransform _randomlocation "0, 0, 0" "1.000000,1.000000,1.000000") "AdjustIfPossibleButAlwaysSpawn" "MultiplyWithRoot" 0 0))
      (bind _asbp_enemy_base (Utilities|Casting|CastToBP_Enemy_Base _returnvalue))
      (Variables|/Game/ForgettenRealms/Enemies/Blueprint/BaseEnemies/BP_Enemy_Base.BP_Enemy_Base_C|SetOrigin _asbp_enemy_base self)
      (Math|Integer|IncrementInt (Variables|Default|GetCurrentSpawnCount)
        (:%20%20
          (if (== (Variables|Default|GetSpawnerActorType) "/Game/ForgettenRealms/Enemies/Blueprint/Centaur/BP_Enemy_Melee_Centaur.BP_Enemy_Melee_Centaur_C")
            (Variables|/Game/ForgettenRealms/Enemies/Blueprint/BaseEnemies/BP_Enemy_Base.BP_Enemy_Base_C|SetOriginDistance _asbp_enemy_base 5e+03)
            ;[1 1 1] Spawn 2 centaurs around the original one
            (CallFunction|SpawnMinions (Transformation|GetActorLocation _returnvalue))
            (CallFunction|SpawnMinions (Transformation|GetActorLocation _returnvalue)))
          (if (Variables|Default|GetFirstSpawn?)
            ;[1 1 1] Continue to spawn the first wave (On begin play)
            (CallFunction|FirstSpawn)
            (else
              ;[1 1 1] Respawn Enemies as Normal
              (CallFunction|RespawnEnemies)))))
      (else
        (Variables|Default|SetCanRespawn? false)
        (Variables|Default|SetFirstSpawn? false)))))

(event Custom|SpawnMinions
  (params (ParentLocation :type Vector))
  (bind _randomlocation (Class|NavigationSystemV1|GetRandomLocationinNavigableRadius ParentLocation 3.5e+02 0 0))
  (bind _returnvalue (Game|SpawnActorfromClass (Variables|Default|GetSpawnerActorType) (Math|Transform|MakeTransform _randomlocation "0, 0, 0" "1.000000,1.000000,1.000000") "AdjustIfPossibleButAlwaysSpawn" "MultiplyWithRoot" 0 0))
  (bind _asbp_enemy_base (Utilities|Casting|CastToBP_Enemy_Base _returnvalue))
  (Variables|/Game/ForgettenRealms/Enemies/Blueprint/BaseEnemies/BP_Enemy_Base.BP_Enemy_Base_C|SetOrigin _asbp_enemy_base self)
  (Variables|/Game/ForgettenRealms/Enemies/Blueprint/BaseEnemies/BP_Enemy_Base.BP_Enemy_Base_C|SetOriginDistance _asbp_enemy_base 5e+03))

(event EventBeginPlay
  (CallFunction|FirstSpawn))

(event EventTick
  (params (DeltaSeconds :type Float%20%28single-precision%29)))

(fn ConstructionScript
  (if (Variables|Default|GetShortenRadius?)
    (Components|Sphere|SetSphereRadius (Variables|Default|GetCullRespawnRadius) 6.5e+03 true)))

(fn ShortenRadius)