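; Wolf melee enemy, a child Blueprint that uses Barghest meshes and adds its attack and damage hooks to the parent's behavior.
; On BeginPlay, after the parent's logic, the tail and mane meshes follow the main mesh's pose via leader pose component.
; The attacking interface event passes the attack montages to the Attacking function.
; Any actor that begins overlapping the melee attack box takes base damage, with no filtering in this graph.
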(event OnComponentBeginOverlap(MeleeAttackBox)
  (params (OverlappedComponent :type Primitive%20Component%20Object%20Reference) (OtherActor :type Actor%20Object%20Reference) (OtherComp :type Primitive%20Component%20Object%20Reference) (OtherBodyIndex :type Integer) (bFromSweep :type Boolean) (SweepResult :type Hit%20Result%20Structure%20%28by%20ref%29))
  (Game|Damage|ApplyDamage OtherActor (Variables|Default|GetBase%20Damage) 0 0))

(event EventBeginPlay
  (|CallParentFunction)
  ;[1 1 1] Make the optional meshes to use the same skeleton as Barghest
  (Components|SkinnedMesh|SetLeaderPoseComponent (Variables|Default|GetSK_BARGHEST_TAIL) (Variables|Character|GetMesh) false false))

(event Collision|EventActorBeginOverlap
  (params (OtherActor :type Actor%20Object%20Reference))
  (|CallParentFunction OtherActor) ; This node is disabled and will not be called.\nDrag off pins to build functionality.
)

(event EventTick
  (params (DeltaSeconds :type Float%20%28single-precision%29))
  (|CallParentFunction DeltaSeconds) ; This node is disabled and will not be called.\nDrag off pins to build functionality.
)

(event EventINTAttacking
  (CallFunction|Attacking (Variables|Default|GetAttack%20Montages)))

(fn ConstructionScript
  (|CallParentFunction))