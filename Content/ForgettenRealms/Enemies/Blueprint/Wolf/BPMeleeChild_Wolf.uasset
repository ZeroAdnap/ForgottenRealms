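; Wolf melee enemy, a child Blueprint that specializes its parent with wolf animations, movement speeds and sounds.
; Optional Barghest tail and mane meshes follow the main mesh's pose through leader pose components.
; Attacks randomly pick a standard or jump attack, while health component hits play a montage that restores walking movement on completion.
; Idle and run events set walk speed, and footstep events alternate two pitched-down sounds.
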(event HitAnim(BPC_Enemy_Health)
  ;[1 1 1] Damage
  (Animation|Montage|PlayMontage (Variables|Character|GetMesh) "/Game/ForgettenRealms/Enemies/Animation/Wolf/AM_Wolf_Hit.AM_Wolf_Hit"
    (:OnCompleted
      (Pawn|Components|CharacterMovement|SetMovementMode (Variables|Character|GetCharacterMovement) "MOVE_Walking" 0))))

(event EventBeginPlay
  (|CallParentFunction)
  ;[1 1 1] Make the optional meshes to use the same skeleton as Barghest
  (Components|SkinnedMesh|SetLeaderPoseComponent (Variables|Default|GetSK_BARGHEST_TAIL) (Variables|Character|GetMesh) false false))

(event EventFootstep
  (switch int (Variables|Default|GetFootstepCount)
    (:0
      (Variables|Default|SetFootstepSound "/Game/ForgettenRealms/Enemies/SFX/Footstep1_Wolf.Footstep1_Wolf")
      (Math|Integer|IncrementInt (Variables|Default|GetFootstepCount)
        (:%20%20
          _)))
    (:1
      (Variables|Default|SetFootstepSound "/Game/ForgettenRealms/Enemies/SFX/Footstep2_Wolf.Footstep2_Wolf")
      (Variables|Default|SetFootstepCount 0)))
  (Audio|PlaySoundatLocation (Variables|Default|GetFootstepSound) (Transformation|GetActorLocation) "0, 0, 0" 1.0 0.6 0.0 0 0 0 0))

(event EventChangeSpeedRun
  (Variables|/Script/Engine.CharacterMovementComponent|SetMaxWalkSpeed (Variables|Character|GetCharacterMovement) 1.1e+03))

(event EventINTAttacking
  (CallFunction|Attacks (Utilities|Select :Index (Math|Random|RandomIntegerinRange 0 1) :Option%200 (Variables|Default|GetAttack%20Anim) :Option%201 (Variables|Default|GetJump%20Attack%20Anim))))

(event EventTick
  (params (DeltaSeconds :type Float%20%28single-precision%29))
  (|CallParentFunction DeltaSeconds) ; This node is disabled and will not be called.\nDrag off pins to build functionality.
)

(event EventChangeSpeedIdle
  (Variables|/Script/Engine.CharacterMovementComponent|SetMaxWalkSpeed (Variables|Character|GetCharacterMovement) 5e+02))

(fn ConstructionScript
  (|CallParentFunction)
  (Variables|Default|SetDeathAnimation "/Game/ForgettenRealms/Enemies/Animation/Wolf/AM_Wolf_Death.AM_Wolf_Death"))