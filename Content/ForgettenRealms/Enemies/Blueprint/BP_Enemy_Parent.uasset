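; Base enemy Blueprint that shows a world-placed health bar and removes itself on death.
; BPC_Enemy_Health supplies the health values and events: damage refreshes the cached WB_Health widget, and death destroys the actor.
; On Tick the widget component turns in yaw only to face the player camera.
; A mesh physics-simulation call exists but is never executed.
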(event Death(BPC_Enemy_Health)
  ;[1 1 1] Death
  (Actor|DestroyActor))

(event ReceivingDamage(BPC_Enemy_Health)
  (bind _bpc_enemy_health (Variables|Default|GetBPC_Enemy_Health))
  ;[1 1 1] Damage
  (Default|SetHealth (Variables|Default|GetAs%20WB%20Health) (Variables|/Game/ForgettenRealms/Enemies/Blueprint/BPC_Enemy_Health.BPC_Enemy_Health_C|GetMax%20Health _bpc_enemy_health) (Variables|/Game/ForgettenRealms/Enemies/Blueprint/BPC_Enemy_Health.BPC_Enemy_Health_C|GetHealth _bpc_enemy_health)))

(event EventTick
  (params (DeltaSeconds :type Float%20%28single-precision%29))
  (Utilities|HealthBarLookatPlayer))

(event EventBeginPlay
  (bind _bpc_enemy_health (Variables|Default|GetBPC_Enemy_Health))
  (bind _aswb_health (Utilities|Casting|CastToWB_Health (UserInterface|GetWidget (Variables|Default|GetWidget))))
  (bind _output_get (Variables|Default|SetAs%20WB%20Health _aswb_health))
  (Default|SetHealth _output_get (Variables|/Game/ForgettenRealms/Enemies/Blueprint/BPC_Enemy_Health.BPC_Enemy_Health_C|GetMax%20Health _bpc_enemy_health) (Variables|/Game/ForgettenRealms/Enemies/Blueprint/BPC_Enemy_Health.BPC_Enemy_Health_C|GetHealth _bpc_enemy_health)))

(fn ConstructionScript)