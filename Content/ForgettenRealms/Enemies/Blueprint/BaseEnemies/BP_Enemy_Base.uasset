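; Base enemy character that handles health feedback, combat, movement speed and death for AI-driven enemies.
; Tick turns the health bar toward the camera and writes zone-leash state to the Blackboard, which also receives enemy type and player target.
; Montage arrays drive combo attacks, while damage briefly stops movement and overlaps toggle a stencil and overlay highlight.
; Health component death stops AI, decrements arena spawner counts, plays a montage or ragdolls, and awards player XP.
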(event DeathAnim(BPC_Enemy_Health)
  ;[1 1 1] Death
)

(event OnComponentBeginOverlap(Stillinrange)
  (params (OverlappedComponent :type Primitive%20Component%20Object%20Reference) (OtherActor :type Actor%20Object%20Reference) (OtherComp :type Primitive%20Component%20Object%20Reference) (OtherBodyIndex :type Integer) (bFromSweep :type Boolean) (SweepResult :type Hit%20Result%20Structure%20%28by%20ref%29))
  (CallFunction|SetPlayerStillinRange))

(event Death(BPC_Enemy_Health)
  (bind _deathanimation (Variables|Default|GetDeathAnimation))
  ;[1 1 1] Death
  (Utilities|FlowControl|Sequence
    (:then_0
      ;;[1 1 1] Stop Enemy Movement and AI Logic
      (Class|NavMovementComponent|StopMovementKeepPathing (Variables|Character|GetCharacterMovement))
      (AI|Logic|StopLogic (Variables|/Script/AIModule.AIController|GetBrainComponent (AI|GetAIController self)) "Dead"))
    (:then_1
      ;;[1 1 1] Hide the widget and remove capsule collision
      (Rendering|SetVisibility (Variables|Default|GetWidget) false false)
      (Collision|SetCollisionResponsetoChannel (Variables|Character|GetMesh) "ECC_GameTraceChannel3" "ECR_Overlap"))
    (:then_2
      ;;[1 1 1] If the enemy was spawned in the colloseum, down the enemy left count
      (if (Variables|EnemyType|GetArenaEnemy?)
        (bind _asbpchild_enemy_spawner (Utilities|Casting|CastToBPChild_EnemySpawner (Variables|Default|GetOrigin)))
        (Math|Integer|DecrementInt (Variables|/Game/ForgettenRealms/Enemies/Blueprint/Spawners/BPChild_EnemySpawner.BPChild_EnemySpawner_C|GetEnemyCount _asbpchild_enemy_spawner))))
    (:then_3
      ;;[1 1 1] Is there a death animation?
      (Utilities|IsValid _deathanimation
        (:Is%20Valid
          ;;[1 1 1] Play the death animation
          (Animation|Montage|PlayMontage (Variables|Character|GetMesh) _deathanimation))
        (:Is%20Not%20Valid
          ;;[1 1 1] Simulate physics instead
          (Physics|SetSimulatePhysics (Variables|Character|GetMesh) true)
          (Utilities|FlowControl|Delay 3.0)
          ;;[1 1 1] Destroy actor manually (no notify)
          (Actor|DestroyActor))))
    (:then_4
      ;;[1 1 1] Increase player XP
      (Default|IncreaseXP (Variables|/Game/ForgettenRealms/Player/BP_WukongPlayer.BP_WukongPlayer_C|GetBP_PlayerStat (Variables|Default|GetAs%20BP%20Wukong%20Player)) (Variables|Default|GetAdded%20XP)))))

(event ReceivingDamage(BPC_Enemy_Health)
  (bind _bpc_enemy_health (Variables|Default|GetBPC_Enemy_Health))
  ;[1 1 1] Damage
  (bind _returnvalue (UserInterface|CreateWidget "/Game/ForgettenRealms/Enemies/UI/WB_DamageEnemy.WB_DamageEnemy_C" 0 self (Variables|/Game/ForgettenRealms/Enemies/Blueprint/Component/BPC_Enemy_Health.BPC_Enemy_Health_C|Getdamage (Variables|Default|GetBPC_Enemy_Health))))
  (UserInterface|Viewport|AddtoViewport _returnvalue 0)
  (Default|SetHealth (Variables|Widght|GetAs%20WB%20Health) (Variables|/Game/ForgettenRealms/Enemies/Blueprint/Component/BPC_Enemy_Health.BPC_Enemy_Health_C|GetMax%20Health _bpc_enemy_health) (Variables|/Game/ForgettenRealms/Enemies/Blueprint/Component/BPC_Enemy_Health.BPC_Enemy_Health_C|GetHealth _bpc_enemy_health))
  (Pawn|Components|CharacterMovement|DisableMovement (Variables|Character|GetCharacterMovement))
  (Utilities|FlowControl|Delay 0.4)
  (Pawn|Components|CharacterMovement|SetMovementMode (Variables|Character|GetCharacterMovement) "MOVE_Walking" 0))

(event Custom|RotateActorInDirection
  ;[1 1 1] Rotation
  (Class|Actor|AddActorWorldRotation (Math|Rotator|MakeRotator 0.0 0.0 (* (* (Variables|Rotation|GetRotationSpeed) (Utilities|Time|GetWorldDeltaSeconds)) (Variables|Rotation|GetRotationDircetion)))))

(event Custom|DestroySelf
  ;[1 1 1] Destroy actor on command
  (Actor|DestroyActor))

(event Custom|Attacks
  (params (AttackAnim :type Array%20of%20STRUCT%20Attack%20Anim%20Structures))
  (bind _combo_hit_count (Variables|Default|GetCombo%20hit%20count))
  (bind _charactermovement (Variables|Character|GetCharacterMovement))
  (bind _output (Utilities|Array|Get(acopy) AttackAnim _combo_hit_count))
  ;[1 1 1] Attack function
  (Variables|Default|SetComboAmount (Utilities|Array|Length AttackAnim))
  (if (Utilities|Array|IsValidIndex AttackAnim _combo_hit_count)
    (Animation|Montage|PlayMontage (Variables|Character|GetMesh) (.montages _output) (.playrate _output) (.startposition _output)
      (:then
        (Pawn|Components|CharacterMovement|DisableMovement _charactermovement))
      (:OnCompleted
        (Pawn|Components|CharacterMovement|SetMovementMode _charactermovement "MOVE_Walking" 0)
        (bind _result (Math|Integer|IncrementInt (Variables|Default|GetCombo%20hit%20count))
          (:%20%20
            (if (>= _result (Variables|Default|GetComboAmount))
              (Class|BPIEnemy|INTDoneAttack(Message) self)))))
      (:OnInterrupted
        (Class|BPIEnemy|INTDoneAttack(Message) self)
        (Pawn|Components|CharacterMovement|SetMovementMode (Variables|Character|GetCharacterMovement) "MOVE_Walking" 0)))))

(event Custom|SetEnemyType
  (params (EnemyType :type Byte :default 0) (KeyName :type Name%20%28by%20ref%29) (ControlledActor :type Actor%20Object%20Reference))
  (bind _returnvalue (AI|GetAIController ControlledActor))
  ;[1 1 1] Set Enemy Type
  (if (Utilities|IsValid _returnvalue)
    (Variables|EnemyType|SetEnemyType EnemyType)
    (AI|Components|Blackboard|SetValueasEnum (Variables|/Script/AIModule.AIController|GetBlackboard _returnvalue) KeyName EnemyType)))

(event Custom|SetRotationDirection
  (params (Direction :type Float%20%28double-precision%29))
  ;[1 1 1] Rotation
  (if (== Direction 0.0)
    (Variables|Rotation|SetRotationDircetion 0.0)
    (else
      (Variables|Rotation|SetRotationDircetion (Math|Float|SelectFloat 1.0 -1.0 (> Direction 0.0))))))

(event Custom|Spawn%20Range%20Attack
  (params (Class :type Actor%20Class%20Reference) (Spawn%20Transform%20Location :type Vector) (Spawn%20Transform%20Rotation :type Rotator) (Spawn%20Transform%20Scale :type Vector))
  ;[1 1 1] SpawnRangeAttack
  (Game|SpawnActorfromClass Class (Math|Transform|MakeTransform Spawn%20Transform%20Location Spawn%20Transform%20Rotation Spawn%20Transform%20Scale) "AlwaysSpawn" "MultiplyWithRoot" 0 0))

(event Custom|Check%20Distance
  (params (Self%20Target :type Actor%20Object%20Reference))
  ;[1 1 1] SpawnRangeAttack
  (if (> (Transformation|GetHorizontalDistanceTo Self%20Target (Variables|Default|GetAs%20BP%20Wukong%20Player)) (Variables|EnemyType|GetDistanceForRangeAttack))
    (Variables|EnemyType|SetRangeAttack? true)
    (else
      (Variables|EnemyType|SetRangeAttack? false))))

(event Custom|SetPlayerStill%20in%20range
  (AI|Components|Blackboard|SetValueasObject (Variables|/Script/AIModule.AIController|GetBlackboard (AI|GetAIController (Components|GetOwner))) (Utilities|Name|MakeLiteralName "thePlayer") (Game|GetPlayerCharacter 0)))

(event EventINTChangingSpeed
  (params (Speed :type Float%20%28double-precision%29))
  ;[1 1 1] Interface
  (Variables|/Script/Engine.CharacterMovementComponent|SetMaxWalkSpeed (Variables|Character|GetCharacterMovement) Speed)
  (Variables|Default|SetSpeedChanged true))

(event EventTick
  (params (DeltaSeconds :type Float%20%28single-precision%29))
  (bind _returnvalue (Utilities|Name|MakeLiteralName "inZone"))
  (bind _returnvalue_2 (Utilities|Name|MakeLiteralName "lastLocationVisited"))
  (bind _self self)
  (bind _returnvalue_3 (AI|GetAIController _self))
  (bind _returnvalue_4 (AI|GetBlackboard _returnvalue_3))
  (Utilities|HealthBarLookatPlayer
    (:Output
      (if (Utilities|TooFarfromZone?)
        (AI|Components|Blackboard|SetValueasBool _returnvalue_4 _returnvalue false)
        (AI|Components|Blackboard|SetValueasBool _returnvalue_4 _returnvalue_2 false)
        (else
          (Utilities|FlowControl|Delay 1.5)
          (AI|Components|Blackboard|SetValueasBool _returnvalue_4 _returnvalue true)
          (AI|Components|Blackboard|SetValueasBool _returnvalue_4 _returnvalue_2 false))))))

(event Collision|EventActorBeginOverlap
  (params (OtherActor :type Actor%20Object%20Reference))
  (bind _mesh (Variables|Character|GetMesh))
  ;[1 1 1] Soft LockOverlap
  (Rendering|SetRenderCustomDepth _mesh true)
  (Rendering|SetCustomDepthStencilValue _mesh 3)
  (Rendering|Material|SetOverlayMaterial (Variables|Character|GetMesh) (Variables|Default|GetOverlayMaterial) :!class /Script/Engine.MeshComponent))

(event EventBeginPlay
  (bind _bpc_enemy_health (Variables|Default|GetBPC_Enemy_Health))
  ;[1 1 1] Eventbegin
  (Utilities|FlowControl|Sequence
    (:then_0
      (bind _aswb_health (Utilities|Casting|CastToWB_Health (UserInterface|GetWidget (Variables|Default|GetWidget))))
      (bind _output_get (Variables|Widght|SetAs%20WB%20Health _aswb_health))
      (Default|SetHealth _output_get (Variables|/Game/ForgettenRealms/Enemies/Blueprint/Component/BPC_Enemy_Health.BPC_Enemy_Health_C|GetMax%20Health _bpc_enemy_health) (Variables|/Game/ForgettenRealms/Enemies/Blueprint/Component/BPC_Enemy_Health.BPC_Enemy_Health_C|GetHealth _bpc_enemy_health)))
    (:then_1
      (bind _asbp_wukong_player (Utilities|Casting|CastToBP_WukongPlayer (Game|Player|GetPlayerPawn 0)))
      (Variables|Default|SetAs%20BP%20Wukong%20Player _asbp_wukong_player))))

(event EventINTDoneAttack
  ;[1 1 1] Interface
  (Variables|Default|SetCombo%20hit%20count 0)
  (Variables|Default|SetComboAmount 0))

(event Collision|EventActorEndOverlap
  (params (OtherActor :type Actor%20Object%20Reference))
  (bind _mesh (Variables|Character|GetMesh))
  ;[1 1 1] Soft LockOverlap
  (Rendering|SetRenderCustomDepth _mesh false)
  (Rendering|SetCustomDepthStencilValue _mesh 0)
  (Rendering|Material|SetOverlayMaterial (Variables|Character|GetMesh) 0 :!class /Script/Engine.MeshComponent))

(event EventChangeSpeedRun
  ;[1 1 1] Interface
  (Variables|/Script/Engine.CharacterMovementComponent|SetMaxWalkSpeed (Variables|Character|GetCharacterMovement) 4.5e+02))

(event EventChangeSpeedIdle
  ;[1 1 1] Interface
  (Variables|/Script/Engine.CharacterMovementComponent|SetMaxWalkSpeed (Variables|Character|GetCharacterMovement) 2e+02))

(fn ConstructionScript)