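; Barehanded skeleton enemy, a child Blueprint that reacts to damage and death from its health component and performs a melee attack.
; Damage updates the health bar and plays a hit montage, while attacking plays an attack montage; both pause movement during playback.
; Death hides the widget, ragdolls the mesh with an impulse, then destroys the actor after a delay.
; Custom events switch walk speed between run and idle.
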(event Death(BPC_Enemy_Health)
  ;[1 1 1] Death
  (Utilities|FlowControl|Sequence
    (:then_0
      (Rendering|SetVisibility (Variables|Default|GetWidget) false false)
      (Pawn|Components|CharacterMovement|DisableMovement (Variables|Character|GetCharacterMovement))
      (Collision|SetCollisionEnabled (Variables|Character|GetMesh) "PhysicsOnly")
      (Physics|SetSimulatePhysics (Variables|Character|GetMesh) true))
    (:then_1
      (Physics|AddImpulse (Variables|Character|GetMesh) (Math|Vector|MakeVector (* (.x (Transformation|GetActorLocation (Game|GetPlayerController 0))) 1e+01) 1e+03 1e+02) "None" false)
      (Utilities|FlowControl|Delay 3.0)
      (Actor|DestroyActor))))

(event ReceivingDamage(BPC_Enemy_Health)
  (bind _bpc_enemy_health (Variables|Default|GetBPC_Enemy_Health))
  ;[1 1 1] Damage
  (Default|SetHealth (Variables|Default|GetAs%20WB%20Health) (Variables|/Game/ForgettenRealms/Enemies/Blueprint/BPC_Enemy_Health.BPC_Enemy_Health_C|GetMax%20Health _bpc_enemy_health) (Variables|/Game/ForgettenRealms/Enemies/Blueprint/BPC_Enemy_Health.BPC_Enemy_Health_C|GetHealth _bpc_enemy_health))
  (Pawn|Components|CharacterMovement|DisableMovement (Variables|Character|GetCharacterMovement))
  (bind _returnvalue (Animation|PlayAnimMontage "/Game/ForgettenRealms/Enemies/Animation/Skeleton/Anim_Hit_Montage.Anim_Hit_Montage" 1.0 "None"))
  (Utilities|FlowControl|Delay _returnvalue)
  (Pawn|Components|CharacterMovement|SetMovementMode (Variables|Character|GetCharacterMovement) "MOVE_Walking" 0))

(event EventBeginPlay
  (|CallParentFunction))

(event Collision|EventActorBeginOverlap
  (params (OtherActor :type Actor%20Object%20Reference)))

(event EventINTAttacking
  (Animation|Montage|PlayMontage (Variables|Character|GetMesh) "/Game/ForgettenRealms/Enemies/Animation/Skeleton/Anim_Attack_1_Montage.Anim_Attack_1_Montage"
    (:then
      (Pawn|Components|CharacterMovement|DisableMovement (Variables|Character|GetCharacterMovement)))
    (:OnCompleted
      (Pawn|Components|CharacterMovement|SetMovementMode (Variables|Character|GetCharacterMovement) "MOVE_Walking" 0))))

(event EventTick
  (params (DeltaSeconds :type Float%20%28single-precision%29))
  (|CallParentFunction DeltaSeconds))

(event EventChangeSpeedRun
  (Variables|/Script/Engine.CharacterMovementComponent|SetMaxWalkSpeed (Variables|Character|GetCharacterMovement) 4.5e+02))

(event EventChangeSpeedIdle
  (Variables|/Script/Engine.CharacterMovementComponent|SetMaxWalkSpeed (Variables|Character|GetCharacterMovement) 2e+02))

(fn ConstructionScript
  (|CallParentFunction))