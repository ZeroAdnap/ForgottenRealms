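; BP_Range_Centaur is a ranged centaur enemy that shoots arrows at the Wukong player.
; Each tick it runs a distance check on top of the parent's tick logic.
; The range attack event triggers the attack with a matching bow animation.
; A separate spawn event launches BP_Arrow from a scene component, rotated toward the player's current location.
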(event EventBeginPlay
  (|CallParentFunction) ; This node is disabled and will not be called.\nDrag off pins to build functionality.
)

(event Collision|EventActorBeginOverlap
  (params (OtherActor :type Actor%20Object%20Reference))
  (|CallParentFunction OtherActor) ; This node is disabled and will not be called.\nDrag off pins to build functionality.
)

(event EventTick
  (params (DeltaSeconds :type Float%20%28single-precision%29))
  (|CallParentFunction DeltaSeconds)
  (CallFunction|CheckDistance self))

(event EventINTRangeAttack
  (CallFunction|Attacks (Variables|Default|GetRange%20Attack))
  (Components|Animation|PlayAnimation (Variables|Default|GetBow) "/Game/ForgettenRealms/Enemies/Animation/Skeleton/Bow/Anim_Bow_Attack.Anim_Bow_Attack" false))

(event EventINTSpawnRangeAttack
  (bind _scene (Variables|Default|GetScene))
  (bind _returnvalue (Transformation|GetWorldTransform _scene))
  (CallFunction|SpawnRangeAttack "/Game/ForgettenRealms/Enemies/Blueprint/Projectiles/BP_Arrow.BP_Arrow_C" (.location _returnvalue) (Math|Rotator|FindLookatRotation (.location _returnvalue) (Transformation|GetActorLocation (Variables|Default|GetAs%20BP%20Wukong%20Player))) "1.000000,1.000000,1.000000"))

(fn ConstructionScript
  (|CallParentFunction))