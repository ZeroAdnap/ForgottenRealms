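; Melee centaur enemy Blueprint that specializes a parent enemy class with centaur-specific animations.
; The construction script sets the centaur death montage after running the parent's script.
; The health component's HitAnim event plays the normal get-hit montage, and the INTAttacking event calls Attacks with the melee attack animation.
; BeginPlay, overlap and Tick are disabled placeholder nodes with no added logic.
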(event HitAnim(BPC_Enemy_Health)
  (Animation|PlayAnimMontage "/Game/ForgettenRealms/Enemies/Animation/Centaur/ANIM_Centaur_GetHitNormal_Montage.ANIM_Centaur_GetHitNormal_Montage" 1.0 "None"))

(event EventBeginPlay
  (|CallParentFunction) ; This node is disabled and will not be called.\nDrag off pins to build functionality.
)

(event Collision|EventActorBeginOverlap
  (params (OtherActor :type Actor%20Object%20Reference))
  (|CallParentFunction OtherActor) ; This node is disabled and will not be called.\nDrag off pins to build functionality.
)

(event EventTick
  (params (DeltaSeconds :type Float%20%28single-precision%29))
  (|CallParentFunction DeltaSeconds) ; This node is disabled and will not be called.\nDrag off pins to build functionality.
)

(event EventINTAttacking
  (CallFunction|Attacks (Variables|Default|GetMelee%20Attack%20Anim)))

(fn ConstructionScript
  (|CallParentFunction)
  (Variables|Default|SetDeathAnimation "/Game/ForgettenRealms/Enemies/Animation/Centaur/ANIM_Centaur_DeathNormal_Montage.ANIM_Centaur_DeathNormal_Montage"))