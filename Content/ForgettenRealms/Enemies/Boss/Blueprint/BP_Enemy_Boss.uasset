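; BP_Enemy_Boss is a mountain dragon boss enemy that extends a parent enemy with claw melee attacks and its own death animations.
; Left and right hitbox events toggle query collision on paired claw boxes, and overlaps on each main box apply BaseDamage.
; The attack interface event plays AttackMontages through Attacking, and the health component's death event plays one of two random montages.
; Take-off, landing and AI state-change logic is present but unconnected.
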(event DeathAnim(BPC_Enemy_Health)
  (Animation|PlayAnimMontage (Utilities|Select :Index (Math|Random|RandomIntegerinRange 0 1) :Option%200 "/Game/ForgettenRealms/Enemies/Boss/Animation/ANIM_MOUNTAIN_DRAGON_death_Montage.ANIM_MOUNTAIN_DRAGON_death_Montage" :Option%201 "/Game/ForgettenRealms/Enemies/Boss/Animation/ANIM_MOUNTAIN_DRAGON_deathHitTheGround_Montage.ANIM_MOUNTAIN_DRAGON_deathHitTheGround_Montage") 1.0 "None"))

(event OnComponentBeginOverlap(LClawAttackBox)
  (params (OverlappedComponent :type Primitive%20Component%20Object%20Reference) (OtherActor :type Actor%20Object%20Reference) (OtherComp :type Primitive%20Component%20Object%20Reference) (OtherBodyIndex :type Integer) (bFromSweep :type Boolean) (SweepResult :type Hit%20Result%20Structure%20%28by%20ref%29))
  ;[1 1 1] Claw Attack
  (Game|Damage|ApplyDamage OtherActor (Variables|Default|GetBase%20Damage) 0 0))

(event OnComponentBeginOverlap(RClawAttackBox)
  (params (OverlappedComponent :type Primitive%20Component%20Object%20Reference) (OtherActor :type Actor%20Object%20Reference) (OtherComp :type Primitive%20Component%20Object%20Reference) (OtherBodyIndex :type Integer) (bFromSweep :type Boolean) (SweepResult :type Hit%20Result%20Structure%20%28by%20ref%29))
  ;[1 1 1] Claw Attack
  (Game|Damage|ApplyDamage OtherActor (Variables|Default|GetBase%20Damage) 0 0))

(event Custom|LClawHitBox
  (params (On/Off :type Boolean))
  (bind _lclawattackbox (Variables|Default|GetLClawAttackBox))
  ;[1 1 1] Claw Attack
  (if On/Off
    (Collision|SetCollisionEnabled _lclawattackbox "QueryOnly")
    (else
      (Collision|SetCollisionEnabled _lclawattackbox "NoCollision"))))

(event Custom|RClawHitBox
  (params (On/Off :type Boolean))
  (bind _rclawattackbox (Variables|Default|GetRClawAttackBox))
  ;[1 1 1] Claw Attack
  (if On/Off
    (Collision|SetCollisionEnabled _rclawattackbox "QueryOnly")
    (else
      (Collision|SetCollisionEnabled _rclawattackbox "NoCollision"))))

(event EventBeginPlay
  (|CallParentFunction)
  (Variables|Default|SetDeathDuration 15.0))

(event EventTick
  (params (DeltaSeconds :type Float%20%28single-precision%29))
  (|CallParentFunction DeltaSeconds) ; This node is disabled and will not be called.\nDrag off pins to build functionality.
)

(event EventINTAttacking
  (CallFunction|Attacking (Variables|Default|GetAttackMontages) 1.0 0.0))

(fn ConstructionScript
  (|CallParentFunction))