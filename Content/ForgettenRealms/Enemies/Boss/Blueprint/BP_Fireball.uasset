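; BP_Fireball is a projectile, filed under the boss enemy, that damages the Wukong player on contact.
; Each Tick it moves by a fixed local offset, SpeedFowardX, without sweep or delta-time scaling.
; Any sphere overlap destroys it, first applying damage if the other actor is the BP_WukongPlayer found by GetActorOfClass.
; A delay from BeginPlay also destroys it after a fixed lifetime.
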(event OnComponentBeginOverlap(Sphere)
  (params (OverlappedComponent :type Primitive%20Component%20Object%20Reference) (OtherActor :type Actor%20Object%20Reference) (OtherComp :type Primitive%20Component%20Object%20Reference) (OtherBodyIndex :type Integer) (bFromSweep :type Boolean) (SweepResult :type Hit%20Result%20Structure%20%28by%20ref%29))
  (Utilities|FlowControl|Sequence
    (:then_0
      (bind _returnvalue (Actor|GetActorOfClass "/Game/ForgettenRealms/Player/BP_WukongPlayer.BP_WukongPlayer_C"))
      (if (== _returnvalue OtherActor)
        (Game|Damage|ApplyDamage _returnvalue 2e+01 0 0)))
    (:then_1
      (Actor|DestroyActor))))

(event EventTick
  (params (DeltaSeconds :type Float%20%28single-precision%29))
  (Transformation|AddActorLocalOffset (Variables|Default|GetSpeedFowardX) false false))

(event EventBeginPlay
  (Utilities|FlowControl|Delay 1e+01)
  (Actor|DestroyActor))

(fn ConstructionScript)